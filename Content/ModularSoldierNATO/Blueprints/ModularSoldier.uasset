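; Modular NATO soldier actor assembled from swappable head, body, vest, legs, boots, backpack and helmet meshes that follow the main mesh via master pose.
; The construction script validates each choice against its part array, allowing empty backpack and helmet slots, and creates dynamic materials.
; Update functions push per-part colors, camo pattern, dirt and weathering into those materials.
; SetNext functions cycle parts and reapply some of these settings.
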(fn `CheckIfChoosenMeshIsValidFunc`
  (params (TargetMesh :type "SkinnedMeshComponent Object Reference") (ChoosenSkeletal :type "SkeletalMesh Object Reference") (ArrayToCompareWith :type "Array of SkeletalMesh Object Reference") (`IsSlotCanBeEnmpty?` :type Boolean))
  (returns (SkeletalToSet :type "SkeletalMesh Object Reference"))
  (bind _returnvalue (`KismetArrayLibrary.Array_Contains` ArrayToCompareWith ChoosenSkeletal))
  (bind _output (`|GetArrayItem` ArrayToCompareWith))
  (if `IsSlotCanBeEnmpty?`
    (if _returnvalue
      _
      (else
        (`SkinnedMeshComponent.SetSkinnedAssetAndUpdate` TargetMesh _output false :!label _label)
        (return _output)))
    (elif (and _returnvalue (`KismetSystemLibrary.IsValid` ChoosenSkeletal))
      _
      (else
        (goto _label))))
  (`SkinnedMeshComponent.SetSkinnedAssetAndUpdate` TargetMesh ChoosenSkeletal false)
  (return ChoosenSkeletal))

(fn `CreateAndSetDynamicMaterialFunc`
  (params (MeshToSetMaterialTo :type "SkinnedMeshComponent Object Reference") (Dynamicmaterial :type "MaterialInstanceDynamic Object Reference (by ref)") (SelectedSkeletal :type "SkeletalMesh Object Reference") (MaterialElementIndex :type Integer))
  (`/Engine/EditorBlueprintResources/StandardMacros.IsValid` SelectedSkeletal
    (:`Is Valid`
      (bind _returnvalue (`KismetMaterialLibrary.CreateDynamicMaterialInstance` (`.MaterialInterface` (break `SkeletalMaterial` (`|GetArrayItem` (`SkeletalMesh.Materials` SelectedSkeletal) MaterialElementIndex)))))
      (`|VariableSetRef` Dynamicmaterial _returnvalue)
      (`PrimitiveComponent.SetMaterial` MeshToSetMaterialTo MaterialElementIndex _returnvalue))))

(fn `SetNextBackpack`
  (bind _currentbackpack (`self.CurrentBackpack`))
  (bind _skeletaltoset (`self.SetNextItemFunc` (`self.Backpack`) (`self.Backpacks`) (`self.CurrentBackpack`)))
  (set `self.CurrentBackpack` _skeletaltoset)
  (`/Engine/EditorBlueprintResources/StandardMacros.IsValid` _currentbackpack
    (:`Is Valid`
      (`self.CreateAndSetDynamicMaterialFunc` (`self.Backpack`) (`self.BackpackDynamat`) _currentbackpack)
      (`self.UpdateBackpackColorSettingsFunc`)
      (`self.UpdateOverallColorSettings_00_Func`))))

(fn `SetNextBodyFunc`
  (bind _skeletaltoset (`self.SetNextItemFunc` (`self.Body`) (`self.Bodys`) (`self.CurrentBody`)))
  (set `self.CurrentBody` _skeletaltoset)
  (`self.CreateAndSetDynamicMaterialFunc` (`self.Body`) (`self.BodyDynamat`) (`self.CurrentBody`))
  (`self.UpdateUniformColorSettingsFunc`)
  (`self.UpdateOverallColorSettings_00_Func`))

(fn `SetNextBootsFunc`
  (bind _skeletaltoset (`self.SetNextItemFunc` (`self.Boot`) (`self.Boots`) (`self.CurrentBoots`)))
  (set `self.CurrentBoots` _skeletaltoset)
  (`self.CreateAndSetDynamicMaterialFunc` (`self.Boot`) (`self.BootDynamat`) (`self.CurrentBoots`))
  (`self.UpdateBootsColorSettingsFunc`)
  (`self.UpdateOverallColorSettings_00_Func`))

(fn `SetNextHeadFunc`
  (bind _mesh (`self.Mesh`))
  (bind _mesh_2 (`self.Mesh`))
  (bind _skeletalmesh (`SkinnedMeshComponent.SkeletalMesh` _mesh_2))
  (`self.SetNextItemFunc` _mesh (`self.Heads`) (`SkinnedMeshComponent.SkeletalMesh` _mesh))
  (`/Engine/EditorBlueprintResources/StandardMacros.IsValid` _skeletalmesh
    (:`Is Valid`
      (`self.CreateAndSetDynamicMaterialFunc` _mesh_2 (`self.HeadDynamat`) _skeletalmesh)
      (`self.CreateAndSetDynamicMaterialFunc` (`self.Helmet`) (`self.HelmetGlassDynamat`) (`self.CurrentHelmet`) 1)
      (`self.UpdateOverallColorSettings_00_Func`))))

(fn `SetNextHelmetFunc`
  (bind _currenthelmet (`self.CurrentHelmet`))
  (bind _skeletaltoset (`self.SetNextItemFunc` (`self.Helmet`) (`self.Helmets`) (`self.CurrentHelmet`)))
  (set `self.CurrentHelmet` _skeletaltoset)
  (`/Engine/EditorBlueprintResources/StandardMacros.IsValid` _currenthelmet
    (:`Is Valid`
      (`self.CreateAndSetDynamicMaterialFunc` (`self.Helmet`) (`self.HelmetDynamat`) _currenthelmet)
      (`self.CreateAndSetDynamicMaterialFunc` (`self.Helmet`) (`self.HelmetGlassDynamat`) (`self.CurrentHelmet`) 1)
      (`self.UpdateHelmetColorSettingsFunc`)
      (`self.UpdateOverallColorSettings_00_Func`))))

(fn `SetNextItemFunc`
  (params (TargetMesh :type "SkinnedMeshComponent Object Reference") (ArrayToCompareWith :type "Array of SkeletalMesh Object Reference") (CurrentSkeletal :type "SkeletalMesh Object Reference"))
  (returns (SkeletalToSet :type "SkeletalMesh Object Reference"))
  (bind _returnvalue (`KismetArrayLibrary.Array_Find` ArrayToCompareWith CurrentSkeletal))
  (bind _output (`|GetArrayItem` ArrayToCompareWith))
  (bind _output_2 (`|GetArrayItem` ArrayToCompareWith (+ _returnvalue 1)))
  (if (> (`KismetArrayLibrary.Array_LastIndex` ArrayToCompareWith) _returnvalue)
    (`SkinnedMeshComponent.SetSkinnedAssetAndUpdate` TargetMesh _output_2 false)
    (return _output_2)
    (else
      (`SkinnedMeshComponent.SetSkinnedAssetAndUpdate` TargetMesh _output false)
      (return _output))))

(fn `SetNextLegsFunc`
  (bind _skeletaltoset (`self.SetNextItemFunc` (`self.Leg`) (`self.Legs`) (`self.CurrentLegs`)))
  (set `self.CurrentLegs` _skeletaltoset)
  (`self.CreateAndSetDynamicMaterialFunc` (`self.Leg`) (`self.LegDynamat`) (`self.CurrentLegs`))
  (`self.UpdateUniformColorSettingsFunc`)
  (`self.UpdateOverallColorSettings_00_Func`))

(fn `SetNextVestFunc`
  (bind _skeletaltoset (`self.SetNextItemFunc` (`self.Vest`) (`self.Vests`) (`self.CurrentVest`)))
  (set `self.CurrentVest` _skeletaltoset)
  (`self.CreateAndSetDynamicMaterialFunc` (`self.Vest`) (`self.VestDynamat`) (`self.CurrentVest`))
  (`self.UpdateVestColorSettingsFunc`)
  (`self.UpdateOverallColorSettings_00_Func`))

(fn `UpdateBackpackColorSettingsFunc`
  (bind _backpackdynamat (`self.BackpackDynamat`))
  (`/Engine/EditorBlueprintResources/StandardMacros.IsValid` (`self.BackpackDynamat`)
    (:`Is Valid`
      (`MaterialInstanceDynamic.SetTextureParameterValue` _backpackdynamat "CamoPattern" (`self.CammoPattern`))
      (`MaterialInstanceDynamic.SetScalarParameterValue` _backpackdynamat "should use camopattern? (1=true, 0=false)" (select `bool` (`self.IsCamoPattern?_(Backpack)`) :`true` 1.0 :!type "Float (single-precision)"))
      (`MaterialInstanceDynamic.SetVectorParameterValue` _backpackdynamat "Fabric1Color(if not camo)" (`self.Fabric1_Color_If_NotCamo_(Backpack)`))
      (`MaterialInstanceDynamic.SetVectorParameterValue` _backpackdynamat "Fabrik2_Color" (`self.Fabric2_Color_(Backpack)`))
      (`MaterialInstanceDynamic.SetVectorParameterValue` _backpackdynamat "Fabrik3_Color" (`self.Fabric3_Color_(Backpack)`))
      (`MaterialInstanceDynamic.SetVectorParameterValue` _backpackdynamat "Fabrik4_Color" (`self.Fabric4_Color_(Backpack)`))
      (`MaterialInstanceDynamic.SetVectorParameterValue` _backpackdynamat "Plastic1Color" (`self.Plastic1Color_(Backpack)`)))))

(fn `UpdateBootsColorSettingsFunc`
  (bind _bootdynamat (`self.BootDynamat`))
  (`MaterialInstanceDynamic.SetVectorParameterValue` _bootdynamat "Leather1_Color" (`self.Leather1_Color_(Boots)`))
  (`MaterialInstanceDynamic.SetVectorParameterValue` _bootdynamat "Leather2_Color" (`self.Leather2_Color_(Boots)`))
  (`MaterialInstanceDynamic.SetVectorParameterValue` _bootdynamat "Fabrik3_Color" (`self.Fabric_Color_(Boots)`))
  (`MaterialInstanceDynamic.SetVectorParameterValue` _bootdynamat "Fabrik4_Color" (`self.Laces_Color_(Boots)`))
  (`MaterialInstanceDynamic.SetVectorParameterValue` _bootdynamat "Plastic1Color" (`self.Sole_Color_(Boots)`))
  (`MaterialInstanceDynamic.SetVectorParameterValue` _bootdynamat "Plastic2Color" (`self.Plastic_Color_(Boots)`))
  (`MaterialInstanceDynamic.SetVectorParameterValue` _bootdynamat "Plastic3Color" (`self.Metal_Color_(Boots)`))
  (`MaterialInstanceDynamic.SetVectorParameterValue` _bootdynamat "MetalColor" (`self.MetalColor_(Vest)`)))

(fn `UpdateHelmetColorSettingsFunc`
  (bind _helmetdynamat (`self.HelmetDynamat`))
  (`/Engine/EditorBlueprintResources/StandardMacros.IsValid` (`self.HelmetDynamat`)
    (:`Is Valid`
      (`MaterialInstanceDynamic.SetTextureParameterValue` _helmetdynamat "CamoPattern" (`self.CammoPattern`))
      (`MaterialInstanceDynamic.SetScalarParameterValue` _helmetdynamat "should use camopattern? (1=true, 0=false)" (select `bool` (`self.IsCamoPattern?_(Helmet)`) :`true` 1.0 :!type "Float (single-precision)"))
      (`MaterialInstanceDynamic.SetVectorParameterValue` _helmetdynamat "Fabric1Color(if not camo)" (`self.Fabric1_Color_If_NotCamo_(Helmet)`))
      (`MaterialInstanceDynamic.SetVectorParameterValue` _helmetdynamat "Fabrik2_Color" (`self.Fabric2_Color_(Helmet)`))
      (`MaterialInstanceDynamic.SetVectorParameterValue` _helmetdynamat "Fabrik3_Color" (`self.Fabric3_Color_(Helmet)`))
      (`MaterialInstanceDynamic.SetVectorParameterValue` _helmetdynamat "Fabrik4_Color" (`self.Fabric4_Color_(Helmet)`))
      (`MaterialInstanceDynamic.SetVectorParameterValue` _helmetdynamat "Plastic1Color" (`self.Plastic1Color_(Helmet)`))
      (`MaterialInstanceDynamic.SetVectorParameterValue` _helmetdynamat "Plastic2Color" (`self.Plastic2Color_(Helmet)`))
      (`MaterialInstanceDynamic.SetVectorParameterValue` _helmetdynamat "PaintedMetal" (`self.PaintedMetalColor_(Helmet)`))
      (`MaterialInstanceDynamic.SetVectorParameterValue` _helmetdynamat "MetalColor" (`self.MetalColor_(Helmet)`)))))

(fn `UpdateOverallColorSettings_00_Func`
  (bind _output_get (set `self.DirtAmount` (`KismetMathLibrary.FClamp` (`self.DirtAmount`) 0.0 1.1)))
  (`MaterialInstanceDynamic.SetScalarParameterValue` (`self.HeadDynamat`) "DirtAmount" _output_get)
  (`MaterialInstanceDynamic.SetScalarParameterValue` (`self.BodyDynamat`) "DirtAmount" _output_get)
  (`MaterialInstanceDynamic.SetScalarParameterValue` (`self.VestDynamat`) "DirtAmount" _output_get)
  (`MaterialInstanceDynamic.SetScalarParameterValue` (`self.LegDynamat`) "DirtAmount" _output_get)
  (`MaterialInstanceDynamic.SetScalarParameterValue` (`self.BootDynamat`) "DirtAmount" _output_get)
  (`MaterialInstanceDynamic.SetVectorParameterValue` (`self.HeadDynamat`) "DirtColor" (`self.DirtColor`))
  (`MaterialInstanceDynamic.SetVectorParameterValue` (`self.BodyDynamat`) "DirtColor" (`self.DirtColor`))
  (`MaterialInstanceDynamic.SetVectorParameterValue` (`self.VestDynamat`) "DirtColor" (`self.DirtColor`))
  (`MaterialInstanceDynamic.SetVectorParameterValue` (`self.LegDynamat`) "DirtColor" (`self.DirtColor`))
  (`MaterialInstanceDynamic.SetVectorParameterValue` (`self.BootDynamat`) "DirtColor" (`self.DirtColor`))
  (bind _output_get_2 (set `self.FabricWeathered` (`KismetMathLibrary.FClamp` (`self.FabricWeathered`) 0.0 1.1)))
  (`MaterialInstanceDynamic.SetScalarParameterValue` (`self.HeadDynamat`) "Fabric_Weathered" _output_get_2)
  (`MaterialInstanceDynamic.SetScalarParameterValue` (`self.BodyDynamat`) "Fabric_Weathered" _output_get_2)
  (`MaterialInstanceDynamic.SetScalarParameterValue` (`self.VestDynamat`) "Fabric_Weathered" _output_get_2)
  (`MaterialInstanceDynamic.SetScalarParameterValue` (`self.LegDynamat`) "Fabric_Weathered" _output_get_2)
  (`MaterialInstanceDynamic.SetScalarParameterValue` (`self.BootDynamat`) "Fabric_Weathered" _output_get_2))

(fn `UpdateOverallColorSettings_01_Func`
  (bind _dirtcolor (`self.DirtColor`))
  (bind _helmetglassdynamat (`self.HelmetGlassDynamat`))
  (`/Engine/EditorBlueprintResources/StandardMacros.IsValid` (`self.HelmetDynamat`)
    (:`Is Valid`
      (bind _output_get (set `self.DirtAmount` (`KismetMathLibrary.FClamp` (`self.DirtAmount`) 0.0 1.1)))
      (`MaterialInstanceDynamic.SetScalarParameterValue` (`self.HelmetDynamat`) "DirtAmount" _output_get)
      (`MaterialInstanceDynamic.SetVectorParameterValue` (`self.HelmetDynamat`) "DirtColor" _dirtcolor)
      (bind _output_get_2 (set `self.FabricWeathered` (`KismetMathLibrary.FClamp` (`self.FabricWeathered`) 0.0 1.1)))
      (`MaterialInstanceDynamic.SetScalarParameterValue` (`self.HelmetDynamat`) "Fabric_Weathered" _output_get_2)
      (`/Engine/EditorBlueprintResources/StandardMacros.IsValid` _helmetglassdynamat
        (:`Is Valid`
          (`MaterialInstanceDynamic.SetScalarParameterValue` _helmetglassdynamat "DirtAmount" (`self.DirtAmount`))
          (`MaterialInstanceDynamic.SetVectorParameterValue` _helmetglassdynamat "DirtColor" _dirtcolor))))))

(fn `UpdateOverallColorSettings_02_Func`
  (`/Engine/EditorBlueprintResources/StandardMacros.IsValid` (`self.BackpackDynamat`)
    (:`Is Valid`
      (bind _output_get (set `self.DirtAmount` (`KismetMathLibrary.FClamp` (`self.DirtAmount`) 0.0 1.1)))
      (`MaterialInstanceDynamic.SetScalarParameterValue` (`self.BackpackDynamat`) "DirtAmount" _output_get)
      (`MaterialInstanceDynamic.SetVectorParameterValue` (`self.BackpackDynamat`) "DirtColor" (`self.DirtColor`))
      (bind _output_get_2 (set `self.FabricWeathered` (`KismetMathLibrary.FClamp` (`self.FabricWeathered`) 0.0 1.1)))
      (`MaterialInstanceDynamic.SetScalarParameterValue` (`self.BackpackDynamat`) "Fabric_Weathered" _output_get_2))))

(fn `UpdateUniformColorSettingsFunc`
  (bind _legdynamat (`self.LegDynamat`))
  (`MaterialInstanceDynamic.SetTextureParameterValue` _legdynamat "CamoPattern" (`self.CammoPattern`))
  (`MaterialInstanceDynamic.SetTextureParameterValue` (`self.BodyDynamat`) "CamoPattern" (`self.CammoPattern`))
  (`MaterialInstanceDynamic.SetScalarParameterValue` (`self.BodyDynamat`) "should use camopattern? (1=true, 0=false)" (select `bool` (`self.IsCamoPattern?_(Uniform)`) :`true` 1.0 :!type "Float (single-precision)"))
  (`MaterialInstanceDynamic.SetScalarParameterValue` _legdynamat "should use camopattern? (1=true, 0=false)" (select `bool` (`self.IsCamoPattern?_(Uniform)`) :`true` 1.0 :!type "Float (single-precision)"))
  (`MaterialInstanceDynamic.SetVectorParameterValue` _legdynamat "Fabric1Color(if not camo)" (`self.Fabric1_Color_If_NotCamo_(Uniform)`))
  (`MaterialInstanceDynamic.SetVectorParameterValue` (`self.BodyDynamat`) "Fabric1Color(if not camo)" (`self.Fabric1_Color_If_NotCamo_(Uniform)`))
  (`MaterialInstanceDynamic.SetVectorParameterValue` _legdynamat "Fabrik2_Color" (`self.Fabric2_Color_(Uniform)`))
  (`MaterialInstanceDynamic.SetVectorParameterValue` (`self.BodyDynamat`) "Fabrik2_Color" (`self.Fabric2_Color_(Uniform)`))
  (`MaterialInstanceDynamic.SetVectorParameterValue` _legdynamat "Fabrik3_Color" (`self.Fabric3_Color_(Uniform)`))
  (`MaterialInstanceDynamic.SetVectorParameterValue` (`self.BodyDynamat`) "Fabrik3_Color" (`self.Fabric3_Color_(Uniform)`))
  (`MaterialInstanceDynamic.SetVectorParameterValue` _legdynamat "Fabrik4_Color" (`self.Fabric4_Color_(Uniform)`))
  (`MaterialInstanceDynamic.SetVectorParameterValue` (`self.BodyDynamat`) "Fabrik4_Color" (`self.Fabric4_Color_(Uniform)`))
  (`MaterialInstanceDynamic.SetVectorParameterValue` _legdynamat "Plastic1Color" (`self.Plastic1Color_(Uniform)`))
  (`MaterialInstanceDynamic.SetVectorParameterValue` (`self.BodyDynamat`) "Plastic1Color" (`self.Plastic1Color_(Uniform)`)))

(fn `UpdateVestColorSettingsFunc`
  (bind _vestdynamat (`self.VestDynamat`))
  (`MaterialInstanceDynamic.SetTextureParameterValue` _vestdynamat "CamoPattern" (`self.CammoPattern`))
  (`MaterialInstanceDynamic.SetScalarParameterValue` _vestdynamat "should use camopattern? (1=true, 0=false)" (select `bool` (`self.IsCamoPattern?_(Vest)`) :`true` 1.0 :!type "Float (single-precision)"))
  (`MaterialInstanceDynamic.SetVectorParameterValue` _vestdynamat "Fabric1Color(if not camo)" (`self.Fabric1_Color_If_NotCamo_(Vest)`))
  (`MaterialInstanceDynamic.SetVectorParameterValue` _vestdynamat "Fabrik2_Color" (`self.Fabric2_Color_(Vest)`))
  (`MaterialInstanceDynamic.SetVectorParameterValue` _vestdynamat "Fabrik3_Color" (`self.Fabric3_Color_(Vest)`))
  (`MaterialInstanceDynamic.SetVectorParameterValue` _vestdynamat "Fabrik4_Color" (`self.Fabric4_Color_(Vest)`))
  (`MaterialInstanceDynamic.SetVectorParameterValue` _vestdynamat "Plastic1Color" (`self.Plastic1Color_(Vest)`))
  (`MaterialInstanceDynamic.SetVectorParameterValue` _vestdynamat "Plastic2Color" (`self.Plastic2Color_(Vest)`))
  (`MaterialInstanceDynamic.SetVectorParameterValue` _vestdynamat "PaintedMetal" (`self.PaintedMetalColor_(Vest)`))
  (`MaterialInstanceDynamic.SetVectorParameterValue` _vestdynamat "MetalColor" (`self.MetalColor_(Vest)`)))

(fn `UserConstructionScript`
  (bind _mesh (`self.Mesh`))
  ;[1 1 1] Synchronizing bodyparts animation
  (`SkinnedMeshComponent.SetLeaderPoseComponent` (`self.Vest`) (`self.Mesh`) false)
  (`SkinnedMeshComponent.SetLeaderPoseComponent` (`self.Leg`) (`self.Mesh`) false)
  (`SkinnedMeshComponent.SetLeaderPoseComponent` (`self.Boot`) (`self.Mesh`) false)
  (`SkinnedMeshComponent.SetLeaderPoseComponent` (`self.Backpack`) (`self.Mesh`) false)
  (`SkinnedMeshComponent.SetLeaderPoseComponent` (`self.Helmet`) (`self.Mesh`) false)
  (`SkinnedMeshComponent.SetLeaderPoseComponent` (`self.Body`) (`self.Mesh`) false)
  ;[1 1 1] Change Head
  (bind _skeletaltoset (`self.CheckIfChoosenMeshIsValidFunc` _mesh (`SkinnedMeshComponent.SkeletalMesh` _mesh) (`self.Heads`)))
  (`self.CreateAndSetDynamicMaterialFunc` _mesh (`self.HeadDynamat`) _skeletaltoset)
  ;[1 1 1] Change Body
  (bind _skeletaltoset_2 (`self.CheckIfChoosenMeshIsValidFunc` (`self.Body`) (`self.CurrentBody`) (`self.Bodys`)))
  (set `self.CurrentBody` _skeletaltoset_2)
  (`self.CreateAndSetDynamicMaterialFunc` (`self.Body`) (`self.BodyDynamat`) (`self.CurrentBody`))
  ;[1 1 1] Change Vest
  (bind _skeletaltoset_3 (`self.CheckIfChoosenMeshIsValidFunc` (`self.Vest`) (`self.CurrentVest`) (`self.Vests`)))
  (set `self.CurrentVest` _skeletaltoset_3)
  (`self.CreateAndSetDynamicMaterialFunc` (`self.Vest`) (`self.VestDynamat`) (`self.CurrentVest`))
  ;[1 1 1] Change Legs
  (bind _skeletaltoset_4 (`self.CheckIfChoosenMeshIsValidFunc` (`self.Leg`) (`self.CurrentLegs`) (`self.Legs`)))
  (set `self.CurrentLegs` _skeletaltoset_4)
  (`self.CreateAndSetDynamicMaterialFunc` (`self.Leg`) (`self.LegDynamat`) (`self.CurrentLegs`))
  ;[1 1 1] Change Boots
  (bind _skeletaltoset_5 (`self.CheckIfChoosenMeshIsValidFunc` (`self.Boot`) (`self.CurrentBoots`) (`self.Boots`)))
  (set `self.CurrentBoots` _skeletaltoset_5)
  (`self.CreateAndSetDynamicMaterialFunc` (`self.Boot`) (`self.BootDynamat`) (`self.CurrentBoots`))
  ;[1 1 1] Change Backpack
  (bind _skeletaltoset_6 (`self.CheckIfChoosenMeshIsValidFunc` (`self.Backpack`) (`self.CurrentBackpack`) (`self.Backpacks`) true))
  (set `self.CurrentBackpack` _skeletaltoset_6)
  (`self.CreateAndSetDynamicMaterialFunc` (`self.Backpack`) (`self.BackpackDynamat`) (`self.CurrentBackpack`))
  ;[1 1 1] Change Helmet
  (bind _skeletaltoset_7 (`self.CheckIfChoosenMeshIsValidFunc` (`self.Helmet`) (`self.CurrentHelmet`) (`self.Helmets`) true))
  (set `self.CurrentHelmet` _skeletaltoset_7)
  (`self.CreateAndSetDynamicMaterialFunc` (`self.Helmet`) (`self.HelmetDynamat`) (`self.CurrentHelmet`))
  (`self.CreateAndSetDynamicMaterialFunc` (`self.Helmet`) (`self.HelmetGlassDynamat`) (`self.CurrentHelmet`) 1)
  ;[1 1 1] Color Settings
  (`self.UpdateVestColorSettingsFunc`) ; Vest Color Settings
  (`self.UpdateHelmetColorSettingsFunc`) ; Helmet Color Settings
  (`self.UpdateBootsColorSettingsFunc`) ; Boots Color Settings
  (`self.UpdateUniformColorSettingsFunc`) ; Uniform Color Settings
  (`self.UpdateBackpackColorSettingsFunc`) ; Backpack Color Settings
  (`self.UpdateOverallColorSettings_00_Func`) ; Overall Color Settings
  (`self.UpdateOverallColorSettings_01_Func`)
  (`self.UpdateOverallColorSettings_02_Func`))