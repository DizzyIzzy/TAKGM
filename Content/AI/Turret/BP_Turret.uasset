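; Turret AI actor that seeks a nearby visible pawn or vehicle and turns its top mesh toward it; no firing logic.
; Tick sphere-overlaps within SensingRange, filters by distance and line trace, and stores Target, though the compared CurrentDistanceLocal is never assigned.
; Rotation runs inside that loop toward the previous Target at constant speed, with clamped pitch and yaw.
; FindBestTarget (incomplete) and UpdateTurretRotation duplicate this logic but are never called.
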(event `self.ReceiveTick`
  (params (DeltaSeconds :type "Float (single-precision)"))
  ;[1 1 1] Find Best Target
  (set `self.BestDistance (local)` (+ (`self.SensingRange`) 1.0))
  (bind _outactors (`KismetSystemLibrary.SphereOverlapActors` (`self.K2_GetActorLocation`) (`self.SensingRange`) (`|MakeArray` "ObjectTypeQuery3" "ObjectTypeQuery5" :!type "EObjectTypeQuery Enum")))
  (for _array_element _outactors
    (if (not (== (`self.TileSetRef`) _array_element))
      (bind _output_get (set `self.CurrentTarget (local)` _array_element))
      (if (or (< (`self.GetDistanceTo` _output_get self) (`self.BestDistance (local)`)) (not (`KismetSystemLibrary.IsValid` (`self.BestTarget (local)`))))
        ;;[1 1 1] Has Line of Sight
        (bind (_outhit _returnvalue) (`KismetSystemLibrary.LineTraceSingle` (`SceneComponent.K2_GetComponentLocation` (`self.StaticMeshTop`)) (`self.K2_GetActorLocation` (`self.CurrentTarget (local)`)) "TraceTypeQuery1" false (`|MakeArray` self (`self.CurrentTarget (local)`) :!type "Actor Object Reference") "None" false))
        (if (not _returnvalue)
          ;[1 1 1] Update Turret Rotation
          (set `self.BestTarget (local)` (`self.CurrentTarget (local)`))
          (set `self.BestDistance (local)` (`self.CurrentDistance (local)`))
          (`self.Target`
            (:`then`
              (bind _output_get_2 (set `self.NewLocalVar_0` (`KismetMathLibrary.RInterpTo_Constant` (`SceneComponent.K2_GetComponentRotation` (`self.StaticMeshTop`)) (`KismetMathLibrary.FindLookAtRotation` (`SceneComponent.K2_GetComponentLocation` (`self.StaticMeshTop`)) (`self.K2_GetActorLocation` (`self.Target`))) DeltaSeconds (`self.RotationSpeed`))))
              (`SceneComponent.K2_SetWorldRotation` (`self.StaticMeshTop`) (`KismetMathLibrary.MakeRotator` (.roll _output_get_2) (`KismetMathLibrary.ClampAngle` (.pitch _output_get_2) -45.0 75.0) (`KismetMathLibrary.ClampAngle` (.yaw _output_get_2) -90.0 90.0)) false false))
            (:`else`))))))
  (set `self.Target` (`self.BestTarget (local)`)))

(fn `FindBestTarget`
  (locals (`BestDistance (local) 1` :type "Float (double-precision)") (`CurrentDistance (local) 1` :type "Float (double-precision)") (`CurrentTarget (local) 1` :type "Actor Object Reference") (`BestTarget (local) 1` :type "Actor Object Reference"))
  ;[1 1 1] Comment
  (set `local.BestDistance (local) 1` (+ (`self.SensingRange`) 1.0))
  (bind _outactors (`KismetSystemLibrary.SphereOverlapActors` (`self.K2_GetActorLocation`) (`self.SensingRange`) (`|MakeArray` "ObjectTypeQuery3" "ObjectTypeQuery5" :!type "EObjectTypeQuery Enum")))
  (for _array_element _outactors
    (bind _output_get (set `local.CurrentTarget (local) 1` _array_element))
    (if (or (< (`self.GetDistanceTo` _output_get self) (`local.BestDistance (local) 1`)) (not (`KismetSystemLibrary.IsValid` (`local.BestTarget (local) 1`))))
      _))
  (set `self.Target` (`local.BestTarget (local) 1`)))

(fn `UpdateTurretRotation`
  (params (DeltaSeconds :type "Float (double-precision)"))
  (locals (`NewLocalVar_0 1` :type "Rotator Structure" :default (struct)))
  (bind _output_get (set `local.NewLocalVar_0 1` (`KismetMathLibrary.RInterpTo_Constant` (`SceneComponent.K2_GetComponentRotation` (`self.StaticMeshTop`)) (`KismetMathLibrary.FindLookAtRotation` (`SceneComponent.K2_GetComponentLocation` (`self.StaticMeshTop`)) (`self.K2_GetActorLocation` (`self.Target`))) (`local.DeltaSeconds`) (`self.RotationSpeed`))))
  (`SceneComponent.K2_SetWorldRotation` (`self.StaticMeshTop`) (`KismetMathLibrary.MakeRotator` (.roll _output_get) (`KismetMathLibrary.ClampAngle` (.pitch _output_get) -45.0 75.0) (`KismetMathLibrary.ClampAngle` (.yaw _output_get) -90.0 90.0)) false false))

(fn `UserConstructionScript`)