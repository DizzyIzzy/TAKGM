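; BP_UDPSender is an actor that broadcasts CoT strings over UDP from the game on a timer.
; Its Start event opens a named socket to the given IP and port, then sets a timer, looping only if startup succeeds, that calls BroadcastCot with screen and log print options.
; Helper functions use the Georeference to convert actor locations or Unreal coordinates into approximate longitude, latitude and height.
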(event `Start`
  (params (IP :type String) (Port :type Integer) (WaitTime :type "Float (double-precision)"))
  (bind _returnvalue (`self.StartUDPSender` "TestSocket_6" IP Port))
  (`KismetSystemLibrary.K2_SetTimerDelegate` (delegate `Send CoT Strings`) WaitTime _returnvalue))

(event `Send CoT Strings`
  (`self.BroadcastCot` (`self.Print to Screen`) (`self.Print to Log`)))

(event `self.ReceiveTick`
  (params (DeltaSeconds :type "Float (single-precision)")))

(fn `transformActorLocationToRealCoord`
  (params (actor :type "Actor Object Reference"))
  (returns (ReturnValue :type "Vector Structure"))
  (return (`CesiumGeoreference.InaccurateTransformUnrealToLongitudeLatitudeHeight` (`|ConvertAsset` (`self.Georeference`)) (`self.K2_GetActorLocation` actor))))

(fn `transformUECoordToRealCoord`
  (params (unrealCoord :type "Vector Structure"))
  (returns (ReturnValue :type "Vector Structure"))
  (return (`CesiumGeoreference.InaccurateTransformUnrealToLongitudeLatitudeHeight` (`|ConvertAsset` (`self.Georeference`)) unrealCoord)))

(fn `UserConstructionScript`)