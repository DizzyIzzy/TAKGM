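; UDP receiver actor that opens a socket on Start and handles incoming TAK Cursor-on-Target messages to position stand-in actors.
; ParseIncomingCot relays each message through BP_UDPSender, then extracts coordinates and UID by substring search.
; It ignores parsed altitude, line-tracing vertically at the georeferenced lat/lon around its own height to place the UID's mapped stand-in.
; Stand-in spawning is disconnected, so unknown UIDs are only relayed.
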(event `self.ReceiveBeginPlay`)

(event `Start`
  (params (IP :type String) (Port :type Integer))
  (`self.StartUDPReceiver` "Receiver_Socket" (`self.IP`) Port))

(event `self.parseIncomingCot`
  (params (message :type String))
  (bind _returnvalue (+ (`KismetStringLibrary.FindSubstring` message "uid=\"" true) 5))
  (bind _returnvalue_2 (+ (`KismetStringLibrary.FindSubstring` message "lat=\"" false false 0) 5))
  (bind _output (`|ConvertAsset` (`self.Georeference`)))
  (bind (_returnvalue_x _returnvalue_y _returnvalue_z) (`KismetMathLibrary.BreakVector` (`CesiumGeoreference.InaccurateTransformUnrealToLongitudeLatitudeHeight` (`|ConvertAsset` (`self.Georeference`)) (`self.K2_GetActorLocation`))))
  (bind _returnvalue_3 (+ (`KismetStringLibrary.FindSubstring` message "lon=\"" true false _returnvalue_2) 5))
  (bind (_value _returnvalue_4) (`BlueprintMapLibrary.Map_Find` (`self.UidToStandInMap`) (`KismetStringLibrary.GetSubstring` message _returnvalue (- (`KismetStringLibrary.FindSubstring` message "\"" true false _returnvalue) _returnvalue))))
  (bind _returnvalue_5 (+ (`KismetStringLibrary.FindSubstring` message "hae=\"" true false _returnvalue_3) 5))
  (bind _returnvalue_6 (`KismetStringLibrary.GetSubstring` message _returnvalue_5 (- (`KismetStringLibrary.FindSubstring` message "\"" true false _returnvalue_5) _returnvalue_5)))
  (bind _returnvalue_7 (`GameplayStatics.GetActorOfClass` "/Game/UDP/BP_UDPSender.BP_UDPSender_C"))
  (`/Engine/EditorBlueprintResources/StandardMacros.IsValid` _returnvalue_7 ; Isn't valid at game end
    (:`Is Valid`
      (bind _returnvalue_8 (`UDPSender.UDPSender_SendString` _returnvalue_7 message)) ; Relay Incoming messages. TAK is not set up to broadcast due to Android limitations
      (set `self.parsed_latitude` (`KismetStringLibrary.Conv_StringToDouble` (`KismetStringLibrary.GetSubstring` message _returnvalue_2 (- (`KismetStringLibrary.FindSubstring` message "\"" true false _returnvalue_2) _returnvalue_2))))
      (set `self.parsed_longitude` (`KismetStringLibrary.Conv_StringToDouble` (`KismetStringLibrary.GetSubstring` message _returnvalue_3 (- (`KismetStringLibrary.FindSubstring` message "\"" true false _returnvalue_3) _returnvalue_3))))
      (set `self.parsed_hae` (`KismetStringLibrary.Conv_StringToDouble` _returnvalue_6))
      (if (`KismetStringLibrary.NotEqual_StrStr` _returnvalue_6 "9999999")
        _
        (else
          _))
      ;[1 1 1] Calculate UE Coord. without parsed HAE, use Line Trace
      (bind _values (`BlueprintMapLibrary.Map_Values` (`self.UidToStandInMap`)))
      (bind _outhit (`KismetSystemLibrary.LineTraceSingle` (`CesiumGeoreference.InaccurateTransformLongitudeLatitudeHeightToUnreal` _output (`KismetMathLibrary.MakeVector` (`self.parsed_longitude`) (`self.parsed_latitude`) (+ _returnvalue_z 2000.0))) (`CesiumGeoreference.InaccurateTransformLongitudeLatitudeHeightToUnreal` _output (`KismetMathLibrary.MakeVector` (`self.parsed_longitude`) (`self.parsed_latitude`) (- _returnvalue_z 2000.0))) "TraceTypeQuery1" true _values))
      (if _returnvalue_4
        (`self.UpdateStandInLocation` (`.Location` (`GameplayStatics.BreakHitResult` _outhit)) _value)))))

(fn `UpdateStandInLocation`
  (params (`New Location` :type "Vector Structure") (StandIn :type "/Game/AI/NPC/StandIn Object Reference"))
  (bind (_sweephitresult _returnvalue) (`self.K2_SetActorLocation` StandIn `New Location` false true))
  (if _returnvalue
    _))

(fn `UserConstructionScript`)